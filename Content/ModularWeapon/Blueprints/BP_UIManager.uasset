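; Manager actor for the modular weapon UI, showing or hiding the main and per-attachment widgets together.
; Init gathers scene actors and widgets, then binds selector button clicks so only the clicked attachment's selector stays open.
; While UI is displayed, a looping timer line-traces from the camera toward each weapon slot.
; Each attachment's button is enabled only when the hit lands near that attachment, a periodic occlusion check instead of Tick.
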(event Custom|BindOnSelectorDisplayButtonClickedEvents
  (for _array_element (Variables|Default|GetAttachment%20Widget%20Ref)
    (EventDispatchers|BindEventtoSelectorDisplayButtonClicked _array_element (delegate Custom|HideAllSelectorsExceptFocusedOne))))

(event Custom|HideAllSelectorsExceptFocusedOne
  (params (AttachmentWidget :type WBP%20Attachment%20Widget%20Object%20Reference))
  (CallFunction|UpdateAttachmentSelectorVisibility AttachmentWidget))

(event EventBeginPlay)

(event Collision|EventActorBeginOverlap
  (params (OtherActor :type Actor%20Object%20Reference)))

(event EventTick
  (params (DeltaSeconds :type Float%20%28single-precision%29)))

(fn ConstructionScript)

(fn Init
  (CallFunction|GetExternalReferences)
  (CallFunction|BindonSelectorDisplayButtonClickedEvents)
  (Utilities|Time|SetTimerbyFunctionName 0 "UpdateSelectorDisplayButtonVisibility" 0.25 true))

(fn HideAllUIElements
  (Variables|Default|SetUIDisplayed false)
  (Widget|SetVisibility (Variables|Default|GetMain%20Widget%20Ref) "Hidden")
  (for _array_element (Variables|Default|GetAttachment%20Widget%20Ref)
    (Widget|SetVisibility _array_element "Hidden")))

(fn DisplayAllUIElements
  (Variables|Default|SetUIDisplayed true)
  (Widget|SetVisibility (Variables|Default|GetMain%20Widget%20Ref) "SelfHitTestInvisible")
  (for _array_element (Variables|Default|GetAttachment%20Widget%20Ref)
    (Widget|SetVisibility _array_element "SelfHitTestInvisible")))

(fn UpdateAttachmentSelectorVisibility
  (params (AttachmentWidgetReference :type WBP%20Attachment%20Widget%20Object%20Reference))
  (for _array_element (Variables|Default|GetAttachment%20Widget%20Ref)
    (if (not (== _array_element AttachmentWidgetReference))
      (Default|HideSelector _array_element))))

(fn UpdateSelectorDisplayButtonVisibility
  (bind _maincameraref (Variables|Default|GetMainCameraRef))
  (bind _returnvalue (Transformation|GetActorLocation _maincameraref))
  (if (Variables|Default|GetUIDisplayed)
    (for (_array_element _array_index) (Variables|Default|GetAttachmentActorsRef)
      (LocalVariables|SetEvaluatedAttachment _array_element)
      (LocalVariables|SetEvaluatedIndex _array_index)
      (bind _outhit (Collision|LineTraceByChannel _returnvalue (+ _returnvalue (* (Math|Vector|Normalize (- (.location (.attslottransform (Utilities|Array|Get(acopy) (Variables|/Game/ModularWeapon/Blueprints/ModularWeapon/BP_ModularWeapon.BP_ModularWeapon_C|GetCurrentAttSlotsParams (Variables|Default|GetModularWeaponRef)) _array_index))) _returnvalue)) 3.5e+02)) "TraceTypeQuery1" false 0 "None"))
      (bind _isindisplayrange (CallFunction|VerifyAttachmentDistancefromRayHit (LocalVariables|GetEvaluatedAttachment) (.Location (Collision|BreakHitResult _outhit))))
      (if _isindisplayrange
        (Default|SetButtonEnabled (Variables|/Game/ModularWeapon/Blueprints/UMG/WBP_AttachmentWidget.WBP_AttachmentWidget_C|GetWBP_UIButton (Utilities|Array|Get(acopy) (Variables|Default|GetAttachment%20Widget%20Ref) (LocalVariables|GetEvaluatedIndex))))
        (else
          (Default|SetButtonDIsabled (Variables|/Game/ModularWeapon/Blueprints/UMG/WBP_AttachmentWidget.WBP_AttachmentWidget_C|GetWBP_UIButton (Utilities|Array|Get(acopy) (Variables|Default|GetAttachment%20Widget%20Ref) (LocalVariables|GetEvaluatedIndex)))))))))

(fn GetExternalReferences
  (bind _outactors (Actor|GetAllActorsOfClass "/Game/ModularWeapon/Blueprints/BP_SceneConfigurator.BP_SceneConfigurator_C"))
  (Variables|Default|SetMain%20Widget%20Ref (Variables|/Game/ModularWeapon/Blueprints/BP_SceneConfigurator.BP_SceneConfigurator_C|GetMainWidgetRef (Utilities|Array|Get(acopy) _outactors)))
  (bind _outactors_2 (Actor|GetAllActorsOfClass "/Game/ModularWeapon/Blueprints/ModularWeapon/BP_Attachment.BP_Attachment_C"))
  (bind _output_get (Variables|Default|SetAttachmentActorsRef _outactors_2))
  (for _array_element _output_get
    (Utilities|Array|Add (Variables|Default|GetAttachment%20Widget%20Ref) (Variables|/Game/ModularWeapon/Blueprints/ModularWeapon/BP_Attachment.BP_Attachment_C|GetAttachmentWidgetRef _array_element))
    (bind _outactors_3 (Actor|GetAllActorsOfClass "/Game/ModularWeapon/Blueprints/ModularWeapon/BP_ModularWeapon.BP_ModularWeapon_C"))
    (Variables|Default|SetModularWeaponRef (Utilities|Array|Get(acopy) _outactors_3))
    (bind _outactors_4 (Actor|GetAllActorsOfClass "/Game/ModularWeapon/Blueprints/BP_MainCamera.BP_MainCamera_C"))
    (Variables|Default|SetMainCameraRef (Utilities|Array|Get(acopy) _outactors_4))))

(fn VerifyAttachmentDistancefromRayHit
  (params (Attachment :type Actor%20Object%20Reference) (HitLocation :type Vector))
  (return (<= (Math|Vector|Distance(Vector) (Transformation|GetActorLocation Attachment) HitLocation) (Variables|Default|GetAttachmentSelectorButtonDisplayDistance))))