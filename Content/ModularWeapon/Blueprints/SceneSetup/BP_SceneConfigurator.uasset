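; Scene controller for a modular weapon configurator that drives camera, UI and Variant Manager switching of body type and HDRI environment.
; Init registers it with the GameMode, caches level variant sets by index, initializes attachments and UI, and views through the main camera.
; Input drives pan, drag-rotate, zoom, turnaround, UI toggles and environment cycling.
; ActivateVariant switches a variant on and notifies its actors; a lookup maps attachment types to their variant sets.
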(event Custom|CancelTurnAround
  ;[1 1 1] TurnAround
  (Default|StopTurnAround (Variables|ExternalReferences|GetMainCameraRef)))

(event Custom|BindMainWidgetEvents
  (EventDispatchers|BindEventtoOnSelection (Variables|UMGReferences|GetBodyTypeSelectorRef) (delegate Custom|ChangeBodyType))
  (Default|InitSelectorButtons (Variables|UMGReferences|GetBodyTypeSelectorRef) (Variables|VariantSets|GetBodyTypeVarSet) (Variables|Default|GetBodyTypeButtonsSize) (Variables|Default|GetBodyTypeButtonsPadding)))

(event Custom|ChangeBodyType
  (params (Index :type Integer))
  (Variant|ActivateVariant (Variables|VariantSets|GetBodyTypeVarSet) Index))

(event EventBeginPlay
  (Init|Init)
  (CallFunction|BindMainWidgetEvents))

(event Input|ActionEvents|InputActionDragMode
  (params (Key :type Key%20Structure))
  ;[1 1 1] CameraMovements
  (:Pressed
    (Variables|Inputs|SetDragModeActive true)
    (CallFunction|CancelTurnAround))
  (:Released
    (Variables|Inputs|SetDragModeActive false)))

(event Input|ActionEvents|InputActionTriggerTurnAround
  (params (Key :type Key%20Structure))
  ;[1 1 1] TurnAround
  (:Pressed
    (Default|InitiateTurnAround (Variables|ExternalReferences|GetMainCameraRef))))

(event Input|ActionEvents|InputActionHide/DisplayAllUIElements
  (params (Key :type Key%20Structure))
  (bind _uimanagerreference (Variables|ExternalReferences|GetUIManagerReference))
  ;[1 1 1] Hide/Display UI
  (:Pressed
    (Utilities|FlowControl|FlipFlop
      (:A
        (Default|HideAllUIElements _uimanagerreference))
      (:B
        (Default|DisplayAllUIElements _uimanagerreference)))))

(event Input|ActionEvents|InputActionShow/HideControls
  (params (Key :type Key%20Structure))
  (bind _mainwidgetref (Variables|UMGReferences|GetMainWidgetRef))
  ;[1 1 1] Show/Hide Controls
  (:Pressed
    (Utilities|FlowControl|FlipFlop
      (:A
        (Default|ShowControls _mainwidgetref))
      (:B
        (Default|HideControls _mainwidgetref)))))

(event Input|ActionEvents|InputActionCycleHDRIEnv
  (params (Key :type Key%20Structure))
  (:Pressed
    (CallFunction|CycleHDRIEnvironment)))

(event Input|ActionEvents|InputActionPanMode
  (params (Key :type Key%20Structure))
  ;[1 1 1] CameraMovements
  (:Pressed
    (Variables|Inputs|SetPanModeActive true)
    (CallFunction|CancelTurnAround))
  (:Released
    (Variables|Inputs|SetPanModeActive false)))

(event Input|AxisEvents|InputAxisMouseMovementX
  (params (AxisValue :type Float%20%28single-precision%29))
  ;[1 1 1] CameraMovements
  (if (Variables|Inputs|GetDragModeActive)
    (Default|RotateCameraAroundTarget (Variables|ExternalReferences|GetMainCameraRef) AxisValue (stale Input|AxisEvents|InputAxisMouseMovementY AxisValue))
    (elif (Variables|Inputs|GetPanModeActive)
      (Default|Pan (Variables|ExternalReferences|GetMainCameraRef) AxisValue (stale Input|AxisEvents|InputAxisMouseMovementY AxisValue)))))

(event Input|AxisEvents|InputAxisMouseMovementY
  (params (AxisValue :type Float%20%28single-precision%29))
  ;[1 1 1] CameraMovements
  (if (Variables|Inputs|GetDragModeActive)
    (Default|RotateCameraAroundTarget (Variables|ExternalReferences|GetMainCameraRef) (stale Input|AxisEvents|InputAxisMouseMovementX AxisValue) AxisValue)
    (elif (Variables|Inputs|GetPanModeActive)
      (Default|Pan (Variables|ExternalReferences|GetMainCameraRef) (stale Input|AxisEvents|InputAxisMouseMovementX AxisValue) AxisValue))))

(event Input|AxisEvents|InputAxisZoom
  (params (AxisValue :type Float%20%28single-precision%29))
  ;[1 1 1] CameraMovements
  (Default|Zoom (Variables|ExternalReferences|GetMainCameraRef) AxisValue))

(fn ConstructionScript)

(fn Init
  (bind _returnvalue (Game|GetPlayerController 0))
  (Utilities|FlowControl|Sequence
    (:then_0
      ;[1 1 1] Set SceneConfigurator reference in GM
      (bind _asgm_modular_weapon_gm (Utilities|Casting|CastToGM_ModularWeaponGM (Game|GetGameMode)))
      (Variables|/Game/ModularWeapon/Blueprints/Global/GM_ModularWeaponGM.GM_ModularWeaponGM_C|SetSceneConfiguratorReference _asgm_modular_weapon_gm self))
    (:then_1
      ;[1 1 1] Init Variant Sets and all BP_Attachments in the level
      (Init|InitVariantSets)
      (bind _outactors (Actor|GetAllActorsOfClass "/Game/ModularWeapon/Blueprints/ModularWeapon/BP_Attachment.BP_Attachment_C"))
      (for _array_element _outactors
        (Default|Init _array_element)))
    (:then_2
      ;[1 1 1] Initialize Main Widget and camera view
      (bind _returnvalue_2 (UserInterface|CreateWidget "/Game/ModularWeapon/Blueprints/UMG/UMGWidgets/WBP_MainWidget.WBP_MainWidget_C"))
      (bind _output_get (Variables|UMGReferences|SetMainWidgetRef _returnvalue_2))
      (UserInterface|Viewport|AddtoViewport _output_get 0)
      (Variables|/Script/Engine.PlayerController|SetbShowMouseCursor _returnvalue true)
      (Input|SetInputModeGameandUI _returnvalue _output_get "DoNotLock" false)
      (Game|Player|SetViewTargetwithBlend _returnvalue (Variables|ExternalReferences|GetMainCameraRef) 0.0 "VTBlend_Linear" 0.0 false))
    (:then_3
      (Variables|UMGReferences|SetBodyTypeSelectorRef (Variables|/Game/ModularWeapon/Blueprints/UMG/UMGWidgets/WBP_MainWidget.WBP_MainWidget_C|GetWBP_BodyTypeSelector (Variables|UMGReferences|GetMainWidgetRef)))
      (bind _outactors_2 (Actor|GetAllActorsOfClass "/Game/ModularWeapon/Blueprints/SceneSetup/BP_UIManager.BP_UIManager_C"))
      (bind _output_get_2 (Variables|ExternalReferences|SetUIManagerReference (Utilities|Array|Get(acopy) _outactors_2)))
      (Default|Init _output_get_2)
      (Init|InitEnvIndex))))

(fn InitVariantSets
  (bind _returnvalue (Class|LevelVariantSetsActor|GetLevelVariantSets (Variables|ExternalReferences|GetLevelVariantActorRef) true))
  (Variables|VariantSets|SetBodyTypeVarSet (Utilities|Struct|MakeSTR_VariantSet (Class|LevelVariantSets|GetVariantSet _returnvalue) 0 true))
  (Variables|VariantSets|SetAttStockVarSet (Utilities|Struct|MakeSTR_VariantSet (Class|LevelVariantSets|GetVariantSet _returnvalue 1) 0 true))
  (Variables|VariantSets|SetAttMuzzleVarSet (Utilities|Struct|MakeSTR_VariantSet (Class|LevelVariantSets|GetVariantSet _returnvalue 2) 0 true))
  (Variables|VariantSets|SetAttSightVarSet (Utilities|Struct|MakeSTR_VariantSet (Class|LevelVariantSets|GetVariantSet _returnvalue 3) 0 true))
  (Variables|VariantSets|SetAttUnderbarrelVarSet (Utilities|Struct|MakeSTR_VariantSet (Class|LevelVariantSets|GetVariantSet _returnvalue 4) 0 true))
  (Variables|VariantSets|SetAttMagazineVarSet (Utilities|Struct|MakeSTR_VariantSet (Class|LevelVariantSets|GetVariantSet _returnvalue 5) 0 true))
  (Variables|VariantSets|SetAttLateralVarSet (Utilities|Struct|MakeSTR_VariantSet (Class|LevelVariantSets|GetVariantSet _returnvalue 6) 0 true))
  (Variables|VariantSets|SetEnvVarSet (Utilities|Struct|MakeSTR_VariantSet (Class|LevelVariantSets|GetVariantSet _returnvalue 7) 0 true))
  (return))

(fn ActivateVariant
  (params (VariantSet :type STR%20Variant%20Set%20Structure) (VariantIndex :type Integer))
  (Class|Variant|Switchon (Class|VariantSet|GetVariant (Utilities|Struct|BreakSTR_VariantSet VariantSet) VariantIndex))
  (bind _structout (Utilities|Struct|SetmembersinSTR_VariantSet VariantSet VariantIndex))
  (Variant|CallVariantActivatedonActors (.variantset _structout) (.currentvariantindex _structout))
  (return))

(fn CallVariantActivatedonActors
  (params (VariantSet :type Variant%20Set%20Object%20Reference) (VariantIndex :type Integer))
  (bind _returnvalue (Class|VariantSet|GetVariant VariantSet VariantIndex))
  ;[1 1 1] Call "OnVariantActivated" for all actors in variant
  (for _index (range 0 (- (Class|Variant|GetNumActors _returnvalue) 1))
    (Class|IActivableVariant|OnVariantActivated(Message) (Class|Variant|GetActor _returnvalue _index)))
  (return))

(fn FindCorrespondingAttachmentVarSet
  (params (AttachmentType :type eAttachmentType%20Enum :default "NewEnumerator0"))
  (Utilities|FlowControl|Sequence
    (:then_0
      (switch Utilities|FlowControl|Switch|SwitchoneAttachmentType AttachmentType
        (:NewEnumerator0
          (LocalVariables|SetVarSetFound (Variables|VariantSets|GetAttStockVarSet)))
        (:NewEnumerator1
          (LocalVariables|SetVarSetFound (Variables|VariantSets|GetAttMuzzleVarSet)))
        (:NewEnumerator2
          (LocalVariables|SetVarSetFound (Variables|VariantSets|GetAttSightVarSet)))
        (:NewEnumerator3
          (LocalVariables|SetVarSetFound (Variables|VariantSets|GetAttUnderbarrelVarSet)))
        (:NewEnumerator4
          (LocalVariables|SetVarSetFound (Variables|VariantSets|GetAttMagazineVarSet)))
        (:NewEnumerator5
          (LocalVariables|SetVarSetFound (Variables|VariantSets|GetAttLateralVarSet)))))
    (:then_1
      (return (LocalVariables|GetVarSetFound)))))

(fn InitEnvIndex
  (Variables|Default|SetEnvMaxIndex (- (Class|VariantSet|GetNumVariants (.variantset (Variables|VariantSets|GetEnvVarSet))) 1)))

(fn CycleHDRIEnvironment
  (if (== (Variables|Default|GetEnvVariantIndex) (Variables|Default|GetEnvMaxIndex))
    (bind _output_get (Variables|Default|SetEnvVariantIndex 0))
    (Variant|ActivateVariant (Variables|VariantSets|GetEnvVarSet) _output_get)
    (else
      (bind _output_get_2 (Variables|Default|SetEnvVariantIndex (+ (Variables|Default|GetEnvVariantIndex) 1)))
      (Variant|ActivateVariant (Variables|VariantSets|GetEnvVarSet) _output_get_2))))