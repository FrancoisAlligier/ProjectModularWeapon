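; Orbit camera actor that circles, zooms and pans around a target point taken from a look-at actor's location.
; Rotate and zoom functions update a stored rotation and range-limited distance, which Tick turns into actor position before aiming the camera at the target.
; Panning moves the target along camera-relative flat axes, clamped to an X/Z box with Y forced to zero.
; An optional turn-around mode auto-rotates horizontally each tick.
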(event EventBeginPlay
  (Init|Init))

(event EventTick
  (params (DeltaSeconds :type Float%20%28single-precision%29))
  (CallFunction|UpdateCameraPosition)
  (CallFunction|LookatTarget)
  (if (Variables|TurnAround|GetShouldTurnAround)
    (TurnAround|UpdateTurnAround)))

(fn ConstructionScript)

(fn Zoom
  (params (zoomDirection :type Float%20%28single-precision%29))
  (Utilities|FlowControl|Sequence
    (:then_0
      (LocalVariables|SetlocZoomDirection zoomDirection)
      (LocalVariables|SetlocCameraLocation (Transformation|GetActorLocation)))
    (:then_1
      (LocalVariables|SetlocNewDistanceToTarget (Math|Vector|Distance(Vector) (Variables|Default|GetCameraTargetPosition) (+ (Transformation|GetActorLocation) (* (Math|Vector|GetForwardVector (Math|Rotator|FindLookatRotation (Transformation|GetActorLocation) (Variables|Default|GetCameraTargetPosition))) (* (* (Variables|ZoomSettings|GetZoomSpeed) (Utilities|Time|GetWorldDeltaSeconds)) (LocalVariables|GetlocZoomDirection))))))
      ;[1 1 1] Only update CurrentDistanceToTarget if NewDistanceToTarget is in set Min and Max distances
      (if (not (or (<= (LocalVariables|GetlocNewDistanceToTarget) (Variables|ZoomSettings|GetMinZoomDistance)) (>= (LocalVariables|GetlocNewDistanceToTarget) (Variables|ZoomSettings|GetMaxZoomDistance))))
        (Variables|Default|SetCurrentDIstanceToTarget (LocalVariables|GetlocNewDistanceToTarget))))))

(fn LookatTarget
  (bind _camera (Variables|Default|GetCamera))
  (Transformation|SetWorldRotation _camera (Math|Rotator|FindLookatRotation (Transformation|GetWorldLocation _camera) (Variables|Default|GetCameraTargetPosition)) false false))

(fn UpdateCameraPosition
  (Transformation|SetActorLocation (+ (* (Math|Vector|GetForwardVector (Variables|Default|GetCurrentCameraRotationToTarget)) (Variables|Default|GetCurrentDIstanceToTarget)) (Variables|Default|GetCameraTargetPosition)) false false))

(fn RotateCameraAroundTarget
  (params (HorizontalInput :type Float%20%28single-precision%29) (VerticalInput :type Float%20%28single-precision%29))
  (bind _horizontalrotation (Rotation|GetHorizontalRotation HorizontalInput))
  (bind _verticalrotation (Rotation|GetVerticalRotation VerticalInput))
  (Variables|Default|SetCurrentCameraRotationToTarget (Math|Rotator|CombineRotators (Rotation|GetLookatRotationfromTarget) (Math|Rotator|CombineRotators _verticalrotation _horizontalrotation))))

(fn GetHorizontalRotation
  (params (HorizontalInput :type Float%20%28single-precision%29))
  (return (Math|Vector|RotatorfromAxisandAngle "0, 0,1.000000" (* HorizontalInput (* (Variables|RotationSettings|GetHorizontalRotationSpeed) (Utilities|Time|GetWorldDeltaSeconds))))))

(fn GetVerticalRotation
  (params (Verticalinput :type Float%20%28single-precision%29))
  (return (Math|Vector|RotatorfromAxisandAngle (Math|Vector|GetRightVector (Rotation|GetLookatRotationfromTarget)) (* Verticalinput (* (Variables|RotationSettings|GetVerticalRotationSpeed) (Utilities|Time|GetWorldDeltaSeconds))))))

(fn GetLookatRotationfromTarget
  (return (Math|Rotator|FindLookatRotation (Variables|Default|GetCameraTargetPosition) (Transformation|GetActorLocation))))

(fn InitiateTurnAround
  (Variables|TurnAround|SetShouldTurnAround true))

(fn UpdateTurnAround
  (Rotation|RotateCameraAroundTarget (* (Variables|TurnAround|GetTurnAroundSpeedRatio) -1.0) 0.0))

(fn StopTurnAround
  (Variables|TurnAround|SetShouldTurnAround false))

(fn Init
  (Variables|Default|SetCameraTargetPosition (Transformation|GetActorLocation (Variables|Default|GetLookAtTargetActor)))
  (Variables|Default|SetCurrentCameraRotationToTarget (Rotation|GetLookatRotationfromTarget))
  (Init|InitPanBoundaries))

(fn InitPanBoundaries
  (bind _cameratargetposition (Variables|Default|GetCameraTargetPosition))
  (Variables|PanSettings|SetPanMaxBoundary_X (+ (.x _cameratargetposition) (Variables|PanSettings|GetPanBoundaryHalfLenght)))
  (Variables|PanSettings|SetPanMinBoundary_X (- (.x _cameratargetposition) (Variables|PanSettings|GetPanBoundaryHalfLenght)))
  (Variables|PanSettings|SetPanMaxBoundary_Z (+ (.z _cameratargetposition) (Variables|PanSettings|GetPanBoundaryHalfHeight)))
  (Variables|PanSettings|SetPanMinBoundary_Z (- (.z _cameratargetposition) (Variables|PanSettings|GetPanBoundaryHalfHeight))))

(fn PanCamera
  (params (HorizontalInput :type Float%20%28single-precision%29) (VerticalInput%20 :type Float%20%28single-precision%29))
  (bind (_rightdirection _updirection) (Pan|GetFlatDirectionCameratoTarget))
  (bind _rightmovement (Pan|GetPanMovementonAxis _rightdirection HorizontalInput))
  (bind _rightmovement_2 (Pan|GetPanMovementonAxis _updirection VerticalInput%20))
  (Variables|Default|SetCameraTargetPosition (+ (+ _rightmovement_2 _rightmovement) (Variables|Default|GetCameraTargetPosition)))
  (Pan|LimitCameraTargetPosition))

(fn GetPanMovementonAxis
  (params (MovementDirection :type Vector) (Input :type Float%20%28single-precision%29))
  (return (* MovementDirection (* (* Input -1.0) (* (Variables|PanSettings|GetPanSpeed) (Utilities|Time|GetWorldDeltaSeconds))))))

(fn GetFlatDirectionCameratoTarget
  (bind _returnvalue (Transformation|GetActorLocation))
  (bind _cameratargetposition (Variables|Default|GetCameraTargetPosition))
  (bind _z (Math|Vector|BreakVector _cameratargetposition))
  (bind _returnvalue_2 (Math|Vector|MakeVector (.x _returnvalue) (.y _returnvalue) _z))
  (bind _returnvalue_3 (- _cameratargetposition _returnvalue_2))
  (bind _returnvalue_4 (Math|Vector|Normalize _returnvalue_3))
  (bind _returnvalue_5 (Math|Conversions|RotationFromXVector _returnvalue_4))
  (return (Math|Vector|GetRightVector _returnvalue_5) (Math|Vector|GetUpVector _returnvalue_5)))

(fn LimitCameraTargetPosition
  (LocalVariables|SetlocWorkingX (.x (Variables|Default|GetCameraTargetPosition)))
  (LocalVariables|SetlocWorkingZ (.z (Variables|Default|GetCameraTargetPosition)))
  (Utilities|FlowControl|Sequence
    (:then_0
      (LocalVariables|SetlocWorkingX (Math|Float|Clamp(Float) (LocalVariables|GetlocWorkingX) (Variables|PanSettings|GetPanMinBoundary_X) (Variables|PanSettings|GetPanMaxBoundary_X))))
    (:then_1
      (LocalVariables|SetlocWorkingZ (Math|Float|Clamp(Float) (LocalVariables|GetlocWorkingZ) (Variables|PanSettings|GetPanMinBoundary_Z) (Variables|PanSettings|GetPanMaxBoundary_Z))))
    (:then_2
      (Variables|Default|SetCameraTargetPosition (Math|Vector|MakeVector (LocalVariables|GetlocWorkingX) 0.0 (LocalVariables|GetlocWorkingZ))))))