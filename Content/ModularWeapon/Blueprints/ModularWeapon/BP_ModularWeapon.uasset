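; Modular weapon actor that exposes six attachment slots (stock, muzzle, sight, underbarrel, magazine, lateral) through selectable slot configurations.
; Construction, BeginPlay and variant activation rebuild the current slot parameters from the active config, then teleport existing attachment actors to matching slots or park unavailable ones below the origin.
; BeginPlay and variant activation also spawn debug placeholder attachments at available slots through temporary helper functions.
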(event EventBeginPlay
  (CallFunction|Init)
  (Utilities|TEMPSpawnAttachments))

(event Collision|EventActorBeginOverlap
  (params (OtherActor :type Actor%20Object%20Reference)))

(event EventTick
  (params (DeltaSeconds :type Float%20%28single-precision%29)))

(event EventOnVariantActivated
  (CallFunction|Init)
  (Utilities|TEMPSpawnAttachments))

(fn ConstructionScript
  (CallFunction|Init))

(fn UpdateCurrentAttSlotsParams
  (bind _attslotsconfigs (Variables|Default|GetAttSlotsConfigs))
  (bind _currentattslotconfigindex (Variables|Default|GetCurrentAttSlotConfigIndex))
  (bind _output (Utilities|Array|Get(acopy) _attslotsconfigs _currentattslotconfigindex))
  (bind (_stockslotparameters _muzzleslotparameters _sightslotparameters _underbarrelslotparameters _magazineslotparameters _lateralslotparameters) (Utilities|Struct|BreakSTR_AttachmentSlotsConfig _output))
  (Utilities|Array|Clear (Variables|Default|GetCurrentAttSlotsParams))
  (Utilities|FlowControl|Sequence
    (:then_0
      (Utilities|Array|Add (Variables|Default|GetCurrentAttSlotsParams) _stockslotparameters))
    (:then_1
      (Utilities|Array|Add (Variables|Default|GetCurrentAttSlotsParams) _muzzleslotparameters))
    (:then_2
      (Utilities|Array|Add (Variables|Default|GetCurrentAttSlotsParams) _sightslotparameters))
    (:then_3
      (Utilities|Array|Add (Variables|Default|GetCurrentAttSlotsParams) _underbarrelslotparameters))
    (:then_4
      (Utilities|Array|Add (Variables|Default|GetCurrentAttSlotsParams) _magazineslotparameters))
    (:then_5
      (Utilities|Array|Add (Variables|Default|GetCurrentAttSlotsParams) _lateralslotparameters))))

(fn Init
  (Utilities|UpdateCurrentAttSlotsParams)
  (CallFunction|TEMPTeleportAtttoSlot))

(fn TEMPSpawnAttachments
  (for _array_element (Variables|Default|GetCurrentAttSlotsParams)
    (if (Utilities|Enum|Equal(Enum) (.AttSlotAvailability (Utilities|Struct|BreakSTR_AttachmentSlotParameters _array_element)) "NewEnumerator0")
      (Game|SpawnActorfromClass "/Game/ModularWeapon/Blueprints/Debug/BP_DBG_PlaceholderAttachment.BP_DBG_PlaceholderAttachment_C" (.AttSlotTransform (Utilities|Struct|BreakSTR_AttachmentSlotParameters _array_element)) "Undefined" 0 0))))

(fn TEMPTeleportAtttoSlot
  (for (_array_element _array_index) (Variables|Attachments|GetAttachmentsActors)
    (if (Utilities|Enum|Equal(Enum) (.attslotavailability (Utilities|Array|Get(acopy) (Variables|Default|GetCurrentAttSlotsParams) _array_index)) "NewEnumerator0")
      (Transformation|SetActorTransform _array_element (.attslottransform (Utilities|Array|Get(acopy) (Variables|Default|GetCurrentAttSlotsParams) _array_index)) false true)
      (else
        (Transformation|SetActorTransform _array_element (Math|Transform|MakeTransform "0, 0,-250.000000" "0, 0, 0" "1,1,1") false true)))))