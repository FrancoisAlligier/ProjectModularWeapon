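; BP_Attachment is a modular weapon attachment actor that switches between the variants in the variant set for its attachment type.
; Init gets the scene configurator from the modular weapon game mode, looks up that variant set and caches its last index.
; Temporary debug input on NumPad 1–6 cycles variants with wraparound when the key matches this attachment's cycle key, activating them through the configurator.
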(event EventBeginPlay)

(event Collision|EventActorBeginOverlap
  (params (OtherActor :type Actor%20Object%20Reference)))

(event EventTick
  (params (DeltaSeconds :type Float%20%28single-precision%29)))

(event Input|KeyboardEvents|NumPadSix
  (params (Key :type Key%20Structure :default "None"))
  (:Pressed
    (Variables|Default|SetTEMP_PressedCycleKey 6)
    (if (== (Variables|Default|GetTEMP_PressedCycleKey) (Variables|Default|GetTEMP_CycleDebugKey))
      (if (== (Variables|Default|GetTEMP_AttIndex) (Variables|Default|GetTEMP_CycleMaxIndex))
        (bind _output_get (Variables|Default|SetTEMP_AttIndex 0))
        (Default|ActivateVariant (Variables|Default|GetSceneConfiguratorReference) (Variables|Default|GetAttachmentVarSet) _output_get)
        (else
          (bind _result (Math|Integer|IncrementInt (Variables|Default|GetTEMP_AttIndex))
            (:%20%20
              (Default|ActivateVariant (Variables|Default|GetSceneConfiguratorReference) (Variables|Default|GetAttachmentVarSet) _result))))))))

(event Input|KeyboardEvents|NumPadOne
  (params (Key :type Key%20Structure :default "None"))
  (:Pressed
    (Variables|Default|SetTEMP_PressedCycleKey 1)
    (if (== (Variables|Default|GetTEMP_PressedCycleKey) (Variables|Default|GetTEMP_CycleDebugKey))
      (if (== (Variables|Default|GetTEMP_AttIndex) (Variables|Default|GetTEMP_CycleMaxIndex))
        (bind _output_get (Variables|Default|SetTEMP_AttIndex 0))
        (Default|ActivateVariant (Variables|Default|GetSceneConfiguratorReference) (Variables|Default|GetAttachmentVarSet) _output_get)
        (else
          (bind _result (Math|Integer|IncrementInt (Variables|Default|GetTEMP_AttIndex))
            (:%20%20
              (Default|ActivateVariant (Variables|Default|GetSceneConfiguratorReference) (Variables|Default|GetAttachmentVarSet) _result))))))))

(event Input|KeyboardEvents|NumPadTwo
  (params (Key :type Key%20Structure :default "None"))
  (:Pressed
    (Variables|Default|SetTEMP_PressedCycleKey 2)
    (if (== (Variables|Default|GetTEMP_PressedCycleKey) (Variables|Default|GetTEMP_CycleDebugKey))
      (if (== (Variables|Default|GetTEMP_AttIndex) (Variables|Default|GetTEMP_CycleMaxIndex))
        (bind _output_get (Variables|Default|SetTEMP_AttIndex 0))
        (Default|ActivateVariant (Variables|Default|GetSceneConfiguratorReference) (Variables|Default|GetAttachmentVarSet) _output_get)
        (else
          (bind _result (Math|Integer|IncrementInt (Variables|Default|GetTEMP_AttIndex))
            (:%20%20
              (Default|ActivateVariant (Variables|Default|GetSceneConfiguratorReference) (Variables|Default|GetAttachmentVarSet) _result))))))))

(event Input|KeyboardEvents|NumPadThree
  (params (Key :type Key%20Structure :default "None"))
  (:Pressed
    (Variables|Default|SetTEMP_PressedCycleKey 3)
    (if (== (Variables|Default|GetTEMP_PressedCycleKey) (Variables|Default|GetTEMP_CycleDebugKey))
      (if (== (Variables|Default|GetTEMP_AttIndex) (Variables|Default|GetTEMP_CycleMaxIndex))
        (bind _output_get (Variables|Default|SetTEMP_AttIndex 0))
        (Default|ActivateVariant (Variables|Default|GetSceneConfiguratorReference) (Variables|Default|GetAttachmentVarSet) _output_get)
        (else
          (bind _result (Math|Integer|IncrementInt (Variables|Default|GetTEMP_AttIndex))
            (:%20%20
              (Default|ActivateVariant (Variables|Default|GetSceneConfiguratorReference) (Variables|Default|GetAttachmentVarSet) _result))))))))

(event Input|KeyboardEvents|NumPadFour
  (params (Key :type Key%20Structure :default "None"))
  (:Pressed
    (Variables|Default|SetTEMP_PressedCycleKey 4)
    (if (== (Variables|Default|GetTEMP_PressedCycleKey) (Variables|Default|GetTEMP_CycleDebugKey))
      (if (== (Variables|Default|GetTEMP_AttIndex) (Variables|Default|GetTEMP_CycleMaxIndex))
        (bind _output_get (Variables|Default|SetTEMP_AttIndex 0))
        (Default|ActivateVariant (Variables|Default|GetSceneConfiguratorReference) (Variables|Default|GetAttachmentVarSet) _output_get)
        (else
          (bind _result (Math|Integer|IncrementInt (Variables|Default|GetTEMP_AttIndex))
            (:%20%20
              (Default|ActivateVariant (Variables|Default|GetSceneConfiguratorReference) (Variables|Default|GetAttachmentVarSet) _result))))))))

(event Input|KeyboardEvents|NumPadFive
  (params (Key :type Key%20Structure :default "None"))
  (:Pressed
    (Variables|Default|SetTEMP_PressedCycleKey 5)
    (if (== (Variables|Default|GetTEMP_PressedCycleKey) (Variables|Default|GetTEMP_CycleDebugKey))
      (if (== (Variables|Default|GetTEMP_AttIndex) (Variables|Default|GetTEMP_CycleMaxIndex))
        (bind _output_get (Variables|Default|SetTEMP_AttIndex 0))
        (Default|ActivateVariant (Variables|Default|GetSceneConfiguratorReference) (Variables|Default|GetAttachmentVarSet) _output_get)
        (else
          (bind _result (Math|Integer|IncrementInt (Variables|Default|GetTEMP_AttIndex))
            (:%20%20
              (Default|ActivateVariant (Variables|Default|GetSceneConfiguratorReference) (Variables|Default|GetAttachmentVarSet) _result))))))))

(fn ConstructionScript)

(fn Init
  (bind _asgm_modular_weapon_gm (Utilities|Casting|CastToGM_ModularWeaponGM (Game|GetGameMode)))
  (Variables|Default|SetSceneConfiguratorReference (Variables|/Game/ModularWeapon/Blueprints/GM_ModularWeaponGM.GM_ModularWeaponGM_C|GetSceneConfiguratorReference _asgm_modular_weapon_gm))
  (CallFunction|InitVariantSets))

(fn InitVariantSets
  (bind _variant_set (Default|FindCorrespondingAttachmentVarSet (Variables|Default|GetSceneConfiguratorReference) (Variables|Default|GetAttachmentType)))
  (Variables|Default|SetAttachmentVarSet _variant_set)
  (CallFunction|TEMPGetCycleMaxIndex))

(fn TEMPGetCycleMaxIndex
  (Variables|Default|SetTEMP_CycleMaxIndex (- (Class|VariantSet|GetNumVariants (.variantset (Variables|Default|GetAttachmentVarSet))) 1)))