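; BP_SceneConfigurator is a level actor that configures a modular weapon scene through Variant Manager variant sets.
; On BeginPlay it registers with the game mode, caches body-type and stock-attachment variant sets, initializes every BP_Attachment and switches to the main camera.
; The B key cycles three body-type variants, switching each on and messaging its actors through OnVariantActivated.
; A lookup maps attachment types to variant sets, currently covering only Stock.
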(event EventBeginPlay
  (CallFunction|Init))

(event Input|KeyboardEvents|B
  (params (Key :type Key%20Structure :default "None"))
  (:Pressed
    (if (== (Variables|Default|GetBodyTypeVarIndex) 2)
      (bind _output_get (Variables|Default|SetBodyTypeVarIndex 0))
      (CallFunction|ActivateVariant (Variables|VariantSets|GetBodyTypeVarSet) _output_get)
      (else
        (bind _result (Math|Integer|IncrementInt (Variables|Default|GetBodyTypeVarIndex))
          (:%20%20
            (CallFunction|ActivateVariant (Variables|VariantSets|GetBodyTypeVarSet) _result)))))))

(fn ConstructionScript)

(fn InitVariantSets
  (bind _returnvalue (Class|LevelVariantSetsActor|GetLevelVariantSets (Variables|ExternalReferences|GetLevelVariantActorReference) false))
  (Variables|VariantSets|SetBodyTypeVarSet (Utilities|Struct|MakeSTR_VariantSet (Class|LevelVariantSets|GetVariantSet _returnvalue) 0))
  (Variables|VariantSets|SetAttStockVarSet (Utilities|Struct|MakeSTR_VariantSet (Class|LevelVariantSets|GetVariantSet _returnvalue 1) 0))
  (return))

(fn ActivateVariant
  (params (VariantSet :type STR%20Variant%20Set%20Structure) (VariantIndex :type Integer))
  (Class|Variant|Switchon (Class|VariantSet|GetVariant (.VariantSet (Utilities|Struct|BreakSTR_VariantSet VariantSet)) VariantIndex))
  (bind _structout (Utilities|Struct|SetmembersinSTR_VariantSet VariantSet VariantIndex))
  (CallFunction|CallVariantActivatedonActors (.variantset _structout) (.currentvariantindex _structout))
  (return))

(fn CallVariantActivatedonActors
  (params (VariantSet :type Variant%20Set%20Object%20Reference) (VariantIndex :type Integer))
  (bind _returnvalue (Class|VariantSet|GetVariant VariantSet VariantIndex))
  ;[1 1 1] Call "OnVariantActivated" for all actors in variant
  (for _index (range 0 (- (Class|Variant|GetNumActors _returnvalue) 1))
    (Class|IActivableVariant|OnVariantActivated(Message) (Class|Variant|GetActor _returnvalue _index)))
  (return))

(fn FindCorrespondingAttachmentVarSet
  (params (AttachmentType :type eAttachmentType%20Enum :default "NewEnumerator0"))
  (Utilities|FlowControl|Sequence
    (:then_0
      (switch Utilities|FlowControl|Switch|SwitchoneAttachmentType AttachmentType
        (:NewEnumerator0
          (LocalVariables|SetVarSetFound (Variables|VariantSets|GetAttStockVarSet)))))
    (:then_1
      (return (LocalVariables|GetVarSetFound)))))

(fn Init
  (Utilities|FlowControl|Sequence
    (:then_0
      ;[1 1 1] Set SceneConfigurator reference in GM
      (bind _asgm_modular_weapon_gm (Utilities|Casting|CastToGM_ModularWeaponGM (Game|GetGameMode)))
      (Variables|/Game/ModularWeapon/Blueprints/GM_ModularWeaponGM.GM_ModularWeaponGM_C|SetSceneConfiguratorReference _asgm_modular_weapon_gm self))
    (:then_1
      (CallFunction|InitVariantSets)
      (bind _outactors (Actor|GetAllActorsOfClass "/Game/ModularWeapon/Blueprints/ModularWeapon/BP_Attachment.BP_Attachment_C"))
      (for _array_element _outactors
        (Default|Init _array_element)))
    (:then_2
      (Game|Player|SetViewTargetwithBlend (Game|GetPlayerController 0) (Variables|ExternalReferences|GetMainCameraReference) 0.0 "VTBlend_Linear" 0.0 false))))