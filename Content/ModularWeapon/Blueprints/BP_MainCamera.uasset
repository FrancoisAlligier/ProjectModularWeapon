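; Orbit camera actor that keeps its camera aimed at a target actor every tick and supports zoom, manual rotation and an automatic turn-around spin.
; Zoom moves along the line to the target, rejecting steps outside the distance limits and storing the new distance.
; Rotation turns the target-to-camera direction by yaw and pitch, then scales it by that distance without adding target location, so it assumes a target at world origin.
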(event EventBeginPlay)

(event Collision|EventActorBeginOverlap
  (params (OtherActor :type Actor%20Object%20Reference)))

(event EventTick
  (params (DeltaSeconds :type Float%20%28single-precision%29))
  (CallFunction|LookatTarget)
  (if (Variables|TurnAround|GetShouldTurnAround)
    (TurnAround|UpdateTurnAround)))

(fn ConstructionScript)

(fn LookatTarget
  (bind _camera (Variables|Default|GetCamera))
  (Transformation|SetWorldRotation _camera (Math|Rotator|FindLookatRotation (Transformation|GetWorldLocation _camera) (Transformation|GetActorLocation (Variables|General|GetLookAtTargetActor))) false false))

(fn Zoom
  (params (zoomDirection :type Float%20%28single-precision%29))
  (Utilities|FlowControl|Sequence
    (:then_0
      (LocalVariables|SetlocZoomDirection zoomDirection)
      (LocalVariables|SetlocCameraLocation (Transformation|GetActorLocation))
      (LocalVariables|SetlocLookAtTargetLocation (Transformation|GetActorLocation (Variables|General|GetLookAtTargetActor))))
    (:then_1
      (LocalVariables|SetlocNewDistanceToTarget (Math|Vector|Distance(Vector) (LocalVariables|GetlocLookAtTargetLocation) (+ (Transformation|GetActorLocation) (* (Math|Vector|GetForwardVector (Math|Rotator|FindLookatRotation (Transformation|GetActorLocation) (Transformation|GetActorLocation (Variables|General|GetLookAtTargetActor)))) (* (* (Variables|ZoomSettings|GetZoomSpeed) (Utilities|Time|GetWorldDeltaSeconds)) (LocalVariables|GetlocZoomDirection))))))
      (if (not (or (<= (LocalVariables|GetlocNewDistanceToTarget) (Variables|ZoomSettings|GetMinZoomDistance)) (>= (LocalVariables|GetlocNewDistanceToTarget) (Variables|ZoomSettings|GetMaxZoomDistance))))
        (Transformation|SetActorLocation (+ (Transformation|GetActorLocation) (* (Math|Vector|GetForwardVector (Math|Rotator|FindLookatRotation (Transformation|GetActorLocation) (Transformation|GetActorLocation (Variables|General|GetLookAtTargetActor)))) (* (* (Variables|ZoomSettings|GetZoomSpeed) (Utilities|Time|GetWorldDeltaSeconds)) (LocalVariables|GetlocZoomDirection)))) false false)
        (Variables|Default|SetCurrentDIstanceToTarget (LocalVariables|GetlocNewDistanceToTarget))))))

(fn RotateCameraAroundTarget
  (params (HorizontalInput :type Float%20%28single-precision%29) (VerticalInput :type Float%20%28single-precision%29))
  (bind _horizontalrotation (Rotation|GetHorizontalRotation HorizontalInput))
  (bind _verticalrotation (Rotation|GetVerticalRotation VerticalInput))
  (Transformation|SetActorLocation (* (Math|Vector|RotateVector (Math|Vector|GetForwardVector (CallFunction|GetLookatRotationfromTarget)) (Math|Rotator|CombineRotators _verticalrotation _horizontalrotation)) (Variables|Default|GetCurrentDIstanceToTarget)) false false))

(fn GetHorizontalRotation
  (params (HorizontalInput :type Float%20%28single-precision%29))
  (return (Math|Vector|RotatorfromAxisandAngle "0, 0,1.000000" (* HorizontalInput (* (Variables|RotationSettings|GetHorizontalRotationSpeed) (Utilities|Time|GetWorldDeltaSeconds))))))

(fn GetVerticalRotation
  (params (Verticalinput :type Float%20%28single-precision%29))
  (return (Math|Vector|RotatorfromAxisandAngle (Math|Vector|GetRightVector (CallFunction|GetLookatRotationfromTarget)) (* Verticalinput (* (Variables|RotationSettings|GetVerticalRotationSpeed) (Utilities|Time|GetWorldDeltaSeconds))))))

(fn GetLookatRotationfromTarget
  (return (Math|Rotator|FindLookatRotation (Transformation|GetActorLocation (Variables|General|GetLookAtTargetActor)) (Transformation|GetActorLocation))))

(fn InitiateTurnAround
  (Variables|TurnAround|SetShouldTurnAround true))

(fn UpdateTurnAround
  (Rotation|RotateCameraAroundTarget (* (Variables|TurnAround|GetTurnAroundSpeedRatio) -1.0) 0.0))

(fn StopTurnAround
  (Variables|TurnAround|SetShouldTurnAround false))