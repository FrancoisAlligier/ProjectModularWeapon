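; BP_DBG_PlaceholderAttachment is a debug stand-in for a modular weapon attachment, with a cube and a text label.
; The construction script writes AttachmentName to the text render.
; ApplyRandomMaterial sets the cube to a random entry from PossibleMaterials, but nothing in this Blueprint calls it.
; The event graph holds only empty default events.
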(event EventBeginPlay)

(event Collision|EventActorBeginOverlap
  (params (OtherActor :type Actor%20Object%20Reference)))

(event EventTick
  (params (DeltaSeconds :type Float%20%28single-precision%29)))

(fn ConstructionScript
  (Rendering|Components|TextRender|SetText (Variables|Default|GetTextRender) (Utilities|Text|ToText(String) (Variables|Default|GetAttachmentName))))

(fn ApplyRandomMaterial
  (Rendering|Material|SetMaterial (Variables|Default|GetCube) 0 (Utilities|Array|Get(acopy) (Variables|Default|GetPossibleMaterials) (Math|Random|RandomIntegerinRange 0 (Utilities|Array|LastIndex (Variables|Default|GetPossibleMaterials))))))